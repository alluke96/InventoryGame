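; BP_Container is an interactable inventory container that the third-person character can open.
; On BeginPlay it copies its Items array into the BPInventoryComponent inventory slot by slot.
; Interacting with it toggles that inventory, and its box collision shows or collapses the character's interactable prompt on overlap.
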(event `self.ReceiveBeginPlay`
  (for (_array_element _array_index) (`self.Items`)
    (`KismetArrayLibrary.Array_Set` (`/Game/InventorySystem/BP_InventoryComponent.Inventory` (`self.BP_InventoryComponent`)) _array_index _array_element)))

(event `/Game/InventorySystem/BPI_InteractInterface.Interact`
  (params (Interacter :type "Actor Object Reference"))
  (cast `/Game/Blueprints/BP_ThirdPersonCharacter` Interacter)
  (`/Game/InventorySystem/BP_InventoryComponent.ToggleInventory` (`self.BP_InventoryComponent`)))

(event `self.BoxCollision.OnComponentBeginOverlap`
  (params (OverlappedComponent :type "PrimitiveComponent Object Reference") (OtherActor :type "Actor Object Reference") (OtherComp :type "PrimitiveComponent Object Reference") (OtherBodyIndex :type Integer) (bFromSweep :type Boolean) (SweepResult :type "HitResult Structure (by ref)"))
  (bind _asbp_third_person_character (cast `/Game/Blueprints/BP_ThirdPersonCharacter` OtherActor))
  (`Widget.SetVisibility` (`/Game/Blueprints/BP_ThirdPersonCharacter.ItemIsInteractable` _asbp_third_person_character) "Visible"))

(event `self.BoxCollision.OnComponentEndOverlap`
  (params (OverlappedComponent :type "PrimitiveComponent Object Reference") (OtherActor :type "Actor Object Reference") (OtherComp :type "PrimitiveComponent Object Reference") (OtherBodyIndex :type Integer))
  (bind _asbp_third_person_character (cast `/Game/Blueprints/BP_ThirdPersonCharacter` OtherActor))
  (`Widget.SetVisibility` (`/Game/Blueprints/BP_ThirdPersonCharacter.ItemIsInteractable` _asbp_third_person_character) "Collapsed"))

(fn `UserConstructionScript`)