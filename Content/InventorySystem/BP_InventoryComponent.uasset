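; Inventory component that opens and closes the player's inventory window through a single toggle function.
; Toggling on creates the window widget bound to this component, adds it centered-aligned and auto-sized to the player controller's HUD canvas at preset anchors, and switches to UI-only input.
; Toggling off removes the window, clears the reference and restores game-only input.
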(fn `ToggleInventory`
  (bind _returnvalue (`GameplayStatics.GetPlayerController` 0))
  (bind _inventorywindow (`self.InventoryWindow`)
    (:`then`
      (`Widget.RemoveFromParent` _inventorywindow)
      ;[0 0 0] Unset
      (set `self.InventoryWindow` null)
      (`WidgetBlueprintLibrary.SetInputMode_GameOnly` _returnvalue))
    (:`else`
      (bind _returnvalue_2 (`|CreateWidget` "/Game/InventorySystem/InventoryUI/WBP_InventoryWindow.WBP_InventoryWindow_C" null self))
      (bind _output_get (set `self.InventoryWindow` _returnvalue_2))
      (bind _asmy_player_controller (cast `/Game/Core/MyPlayerController` _returnvalue))
      (bind _returnvalue_3 (`CanvasPanel.AddChildToCanvas` (`/Game/InventorySystem/InventoryUI/WBP_HUD.HUDCanvas` (`/Game/Core/MyPlayerController.HUDWidget` _asmy_player_controller)) _output_get))
      (`CanvasPanelSlot.SetAutoSize` _returnvalue_3 true)
      (`CanvasPanelSlot.SetAlignment` _returnvalue_3 (0.5 0.5))
      (`CanvasPanelSlot.SetAnchors` _returnvalue_3 (`self.WindowAnchors`))
      (`WidgetBlueprintLibrary.SetInputMode_UIOnlyEx` (`GameplayStatics.GetPlayerController` 0) (`self.InventoryWindow`) "LockAlways"))))