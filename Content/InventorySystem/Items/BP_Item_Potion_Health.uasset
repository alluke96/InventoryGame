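; Health potion item in the inventory system that restores the player's health when used.
; UseItem calls the parent logic, then casts player 0's character to BP_ThirdPersonCharacter and checks whether health is full.
; If full, it only prints a message; otherwise it adds HealthToAdd to Health without clamping and returns true.
; The event graph and construction script add no logic of their own.
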(fn `UseItem`
  (returns (Success :type Boolean))
  (`parent.UseItem`)
  (bind _asbp_third_person_character (cast `/Game/Blueprints/BP_ThirdPersonCharacter` (`GameplayStatics.GetPlayerCharacter` 0)))
  (bind _healthisfull (`/Game/Blueprints/BP_ThirdPersonCharacter.CheckIfHealthIsFull` _asbp_third_person_character))
  (if _healthisfull
    (`KismetSystemLibrary.PrintString` "HEALTH IS FULL" true true (struct :`R` 1.0 :`B` 0.09301 :`A` 1.0))
    (else
      (set `/Game/Blueprints/BP_ThirdPersonCharacter.Health` (+ (`self.HealthToAdd`) (`/Game/Blueprints/BP_ThirdPersonCharacter.Health` _asbp_third_person_character)) _asbp_third_person_character)
      (return true))))

(fn `UserConstructionScript`
  (`parent.UserConstructionScript`))