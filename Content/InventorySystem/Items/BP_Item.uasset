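; BP_Item is a pickup item actor for the inventory system.
; Interact adds one of its item structure to the interacter's BP_InventoryComponent and destroys the actor if that succeeds.
; Its sphere collision shows the ThirdPersonCharacter's interactable prompt on overlap and collapses it when the overlap ends.
; UseItem is a stub that only returns true.
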(event `/Game/InventorySystem/BPI_InteractInterface.Interact`
  (params (Interacter :type "Actor Object Reference"))
  (bind _success (`/Game/InventorySystem/BP_InventoryComponent.AddToInventory` (`self.GetComponentByClass` Interacter "/Game/InventorySystem/BP_InventoryComponent.BP_InventoryComponent_C") (make `/Game/InventorySystem/SSlotStructure` (`self.ItemStructure`) 1)))
  (if _success
    (`self.K2_DestroyActor`)))

(event `self.SphereCollision.OnComponentBeginOverlap`
  (params (OverlappedComponent :type "PrimitiveComponent Object Reference") (OtherActor :type "Actor Object Reference") (OtherComp :type "PrimitiveComponent Object Reference") (OtherBodyIndex :type Integer) (bFromSweep :type Boolean) (SweepResult :type "HitResult Structure (by ref)"))
  (bind _asthird_person_character (cast `/Game/Blueprints/ThirdPersonCharacter` OtherActor))
  (`Widget.SetVisibility` (`/Game/Blueprints/ThirdPersonCharacter.ItemIsInteractable` _asthird_person_character) "Visible"))

(event `self.SphereCollision.OnComponentEndOverlap`
  (params (OverlappedComponent :type "PrimitiveComponent Object Reference") (OtherActor :type "Actor Object Reference") (OtherComp :type "PrimitiveComponent Object Reference") (OtherBodyIndex :type Integer))
  (bind _asthird_person_character (cast `/Game/Blueprints/ThirdPersonCharacter` OtherActor))
  (`Widget.SetVisibility` (`/Game/Blueprints/ThirdPersonCharacter.ItemIsInteractable` _asthird_person_character) "Collapsed"))

(fn `UseItem`
  (returns (Success :type Boolean))
  (return true))

(fn `UserConstructionScript`)