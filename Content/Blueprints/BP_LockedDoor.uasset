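; Lockable door that the third-person character opens and closes with Interact, unlocking permanently if the player has the matching key.
; Box overlap shows the interact prompt, enables input, checks KeyToCheck and opens a Gate; leaving hides the prompt, disables input and closes it.
; A FlipFlop plays or reverses a timeline that lerps the pivot's yaw, while a locked attempt prints a message.
; BeginPlay applies the configured material to the mesh.
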(event `self.ReceiveBeginPlay`
  (`self.OverrideMaterial`))

(event `InputAction|Interact`
  (params (Key :type "Key Structure"))
  ;[0 0 0] Open door if close enough and has a key
  (:`Pressed`
    (if (or (not (`self.IsLocked`)) (stale `self.BoxCollision.OnComponentBeginOverlap` _haskey))
      (set `self.IsLocked` false)
      (`/Engine/EditorBlueprintResources/StandardMacros.Gate` true :!label _label
        (:`Exit`
          ;[0 0 0] Open / Close animation
          (`/Engine/EditorBlueprintResources/StandardMacros.FlipFlop`
            (:`A`
              (bind (_direction _doortrack) (`Timeline|Open/Close Door` :!label _label_2)
                (:`Update`
                  (`SceneComponent.K2_SetRelativeRotation` (`self.RotationPìvot`) (`KismetMathLibrary.MakeRotator` 0.0 0.0 (`KismetMathLibrary.Lerp` (`self.ClosedAngle`) (`self.OpenedAngle`) _doortrack)) false false))))
            (:`B`
              (goto _label_2 :!via `Reverse`)))))
      (else
        ;[1 1 1] If dont have a key or the door is locked
        (`KismetSystemLibrary.PrintString` "THE DOOR IS LOCKED" true true (struct :`R` 1.0 :`B` 0.087688 :`A` 1.0))))))

(event `self.BoxCollision.OnComponentBeginOverlap`
  (params (OverlappedComponent :type "PrimitiveComponent Object Reference") (OtherActor :type "Actor Object Reference") (OtherComp :type "PrimitiveComponent Object Reference") (OtherBodyIndex :type Integer) (bFromSweep :type Boolean) (SweepResult :type "HitResult Structure (by ref)"))
  ;[0 0 0] Open door if close enough and has a key
  (bind _asbp_third_person_character (cast `/Game/Blueprints/BP_ThirdPersonCharacter` OtherActor))
  (`Widget.SetVisibility` (`/Game/Blueprints/BP_ThirdPersonCharacter.ItemIsInteractable` _asbp_third_person_character) "Visible")
  (`self.EnableInput` (`GameplayStatics.GetPlayerController` 0))
  (bind _haskey (`/Game/Blueprints/BP_ThirdPersonCharacter.CheckIfPlayerHasKey` _asbp_third_person_character (`self.Key to Check`)))
  (goto _label :!via `Open`))

(event `self.BoxCollision.OnComponentEndOverlap`
  (params (OverlappedComponent :type "PrimitiveComponent Object Reference") (OtherActor :type "Actor Object Reference") (OtherComp :type "PrimitiveComponent Object Reference") (OtherBodyIndex :type Integer))
  ;[0 0 0] Open door if close enough and has a key
  (bind _asbp_third_person_character (cast `/Game/Blueprints/BP_ThirdPersonCharacter` OtherActor))
  (`Widget.SetVisibility` (`/Game/Blueprints/BP_ThirdPersonCharacter.ItemIsInteractable` _asbp_third_person_character) "Collapsed")
  (`self.DisableInput` (`GameplayStatics.GetPlayerController` 0))
  (goto _label :!via `Close`))

(fn `OverrideMaterial`
  (`PrimitiveComponent.SetMaterial` (`self.StaticMesh`) 0 (`self.Material`)))

(fn `UserConstructionScript`)