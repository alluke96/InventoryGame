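; Spike trap actor that damages the ThirdPersonCharacter while it stands inside the trap's box collision.
; Entering the box stores the character, sets an overlap flag and applies damage immediately, so quick crossings still hurt.
; A looping timer started on BeginPlay repeats the damage at DamageRate while the flag is set; leaving the box clears it.
; A timeline-driven up-and-down movement event is present but disabled.
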(event `self.ReceiveBeginPlay`
  (bind _damagerate (`self.DamageRate`))
  (`KismetSystemLibrary.K2_SetTimerDelegate` (delegate `DealDamage`) _damagerate true _damagerate))

(event `DealDamage`
  (if (`self.IsOverlaping`)
    (`GameplayStatics.ApplyDamage` (`self.ThirdPersonCharacter`) 20.0)))

(event `self.BoxCollision.OnComponentBeginOverlap`
  (params (OverlappedComponent :type "PrimitiveComponent Object Reference") (OtherActor :type "Actor Object Reference") (OtherComp :type "PrimitiveComponent Object Reference") (OtherBodyIndex :type Integer) (bFromSweep :type Boolean) (SweepResult :type "HitResult Structure (by ref)"))
  (bind _asthird_person_character (cast `/Game/Blueprints/ThirdPersonCharacter` OtherActor))
  (set `self.ThirdPersonCharacter` _asthird_person_character)
  (set `self.IsOverlaping` true)
  ;[0 0 0] I had to apply damage whenever its overlaping since it would only do damage after 1 second, so the player could walk across the spikes for one second and would not get hurt
  (`GameplayStatics.ApplyDamage` (`self.ThirdPersonCharacter`) 20.0))

(event `self.BoxCollision.OnComponentEndOverlap`
  (params (OverlappedComponent :type "PrimitiveComponent Object Reference") (OtherActor :type "Actor Object Reference") (OtherComp :type "PrimitiveComponent Object Reference") (OtherBodyIndex :type Integer))
  (cast `/Game/Blueprints/ThirdPersonCharacter` OtherActor)
  (set `self.IsOverlaping` false))

(event `MoveUpAndDown`
  (bind _defaultsceneroot (`self.DefaultSceneRoot`))
  (bind (_returnvalue_x _returnvalue_y) (`KismetMathLibrary.BreakVector` (`SceneComponent.K2_GetComponentLocation` _defaultsceneroot)))
  ;[1 0 0] Disabled
  (`Timeline|MoveUp` :!via `PlayFromStart` :!label _label
    (:`Update`
      (bind (_direction _moveupanddown) (`Timeline|MoveDown` :!via `ReverseFromEnd`)
        (:`Update`
          (`SceneComponent.K2_SetRelativeLocation` _defaultsceneroot (`KismetMathLibrary.MakeVector` _returnvalue_x _returnvalue_y (* _moveupanddown 200.0)) false false))
        (:`Finished`
          (goto _label :!via `PlayFromStart`))))))

(fn `UserConstructionScript`)