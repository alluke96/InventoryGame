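; BP_Dummy is a damageable target dummy actor with a health bar widget.
; Any damage received while Health is above zero lowers it and refreshes the bar; a hit arriving at zero or below destroys the actor.
; UpdateHealthBarMeter, also run on BeginPlay, casts the HealthBar component's widget to WBP_DummyHealthMeter and sets its progress bar from Health, assuming a maximum of 100.
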(event `self.ReceiveBeginPlay`
  (`self.UpdateHealthBarMeter`))

(event `self.ReceiveAnyDamage`
  (params (Damage :type "Float (single-precision)") (DamageType :type "DamageType Object Reference") (InstigatedBy :type "Controller Object Reference") (DamageCauser :type "Actor Object Reference"))
  (if (> (`self.Health`) 0.0)
    (set `self.Health` (- (`self.Health`) Damage))
    (`self.UpdateHealthBarMeter`)
    (else
      (`self.K2_DestroyActor`))))

(fn `UpdateHealthBarMeter`
  (bind _aswbp_dummy_health_meter (cast `/Game/UI/WBP_DummyHealthMeter` (`WidgetComponent.GetUserWidgetObject` (`self.HealthBar`))))
  (`ProgressBar.SetPercent` (`/Game/UI/WBP_DummyHealthMeter.ProgressBar_0` _aswbp_dummy_health_meter) (/ (`self.Health`) 100.0)))

(fn `UserConstructionScript`)